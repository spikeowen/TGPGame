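; AI enemy character that gives hit feedback and can drop loot on death, driven by its HealthComponent events.
; Taking damage spawns a floating damage number and an attached blood emitter, whose particle collisions place randomized, short-lived blood decals through dynamic material instances.
; On death the capsule ignores pawn collision and a one-time random roll may drop an ammo or health pickup.
; No chase logic appears in these graphs.
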(event OnComponentTakeDamage(HealthComponent)
  (params (causer :type Controller%20Object%20Reference) (damage :type Float%20%28single-precision%29))
  (bind _returnvalue (Game|SpawnActorfromClass "/Game/DamageMarkerBPFInal.DamageMarkerBPFInal_C" (Math|Conversions|ToTransform(Vector) (+ (Transformation|GetActorLocation) "0, 0,100.000000")) "Undefined" 0 0))
  (Class|MyDamageMarker|SetSpawnedby _returnvalue causer)
  (Class|MyDamageMarker|SetText _returnvalue (Math|Float|Truncate damage))
  (bind _returnvalue_2 (Effects|SpawnEmitterAttached "/Game/Blood_Splatter/Blood_Particles.Blood_Particles" (Variables|Character|GetMesh) "None" "0, 0,15.000000"))
  (EventDispatchers|BindEventtoOnParticleCollide _returnvalue_2 (delegate Custom|On%20Collide%20Event)))

(event OnComponentDead(HealthComponent)
  (params (causer :type Controller%20Object%20Reference))
  (Collision|SetCollisionResponsetoChannel (Variables|Default|GetCapsuleComponent) "ECC_Pawn" "ECR_Ignore")
  (if (not (Variables|Default|GetHasTriedSpawningPickup))
    (Variables|Default|SetHasTriedSpawningPickup true)
    (bind _output_get (Variables|Default|SetRandomForThisFrame (Math|Random|RandomFloat)))
    (if (> _output_get 0.8)
      (Game|SpawnActorfromClass "/Game/Blueprints/Pickups/AmmoPickup.AmmoPickup_C" (Math|Transform|MakeTransform (Transformation|GetActorLocation) "0, 0, 0" "1,1,1") "Undefined" 0 0)
      (elif (> _output_get 0.6)
        (Game|SpawnActorfromClass "/Game/Blueprints/Pickups/HealthPickupActorBP.HealthPickupActorBP_C" (Math|Transform|MakeTransform (Transformation|GetActorLocation) "0, 0, 0" "1,1,1") "Undefined" 0 0)))))

(event Custom|On%20Collide%20Event
  (params (EventName :type Name) (EmitterTime :type Float%20%28single-precision%29) (ParticleTime :type Integer) (Location :type Vector) (Velocity :type Vector) (Direction :type Vector) (Normal :type Vector) (BoneName :type Name) (PhysMat :type Physical%20Material%20Object%20Reference))
  (bind _returnvalue (Rendering|Material|CreateDynamicMaterialInstance "/Game/Blood_Splatter/Blood_Decal_Material.Blood_Decal_Material" "None" "None" :!class /Script/Engine.KismetMaterialLibrary))
  (Rendering|Material|SetScalarParameterValue _returnvalue "Frame" (Math|Conversions|ToFloat(Integer) (Math|Random|RandomInteger 11)) :!class /Script/Engine.MaterialInstanceDynamic)
  (Rendering|Decal|SpawnDecalatLocation _returnvalue (Math|Conversions|ToVector(Float) (Math|Random|RandomFloatinRange 2e+01 5e+01)) Location (Math|Conversions|RotationFromXVector Normal) 8.0))

(event EventBeginPlay)

(event Collision|EventActorBeginOverlap
  (params (OtherActor :type Actor%20Object%20Reference)))

(event EventTick
  (params (DeltaSeconds :type Float%20%28single-precision%29)))

(event EventSetHealth
  (params (newHealth :type Float%20%28single-precision%29)))

(fn ConstructionScript)