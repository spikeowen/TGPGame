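; BP_AIChaseObjective is an AI pawn that tracks players through perception and gives visual feedback when damaged.
; Perception updates set the sensed BP_BasePlayer as the blackboard "target" and clear it when sensing is lost.
; Damage from its HealthComponent spawns a damage-number marker and an attached blood emitter.
; Blood particle collisions spawn short-lived, surface-aligned decals with random size and material frame through dynamic material instances.
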(event OnComponentTakeDamage(HealthComponent)
  (params (causer :type Controller%20Object%20Reference) (damage :type Float%20%28single-precision%29))
  (bind _returnvalue (Game|SpawnActorfromClass "/Game/DamageMarkerBPFInal.DamageMarkerBPFInal_C" (Math|Conversions|ToTransform(Vector) (+ (Transformation|GetActorLocation) "0, 0,100.000000")) "Undefined" 0 0))
  (Class|MyDamageMarker|SetSpawnedby _returnvalue causer)
  (Class|MyDamageMarker|SetText _returnvalue (Math|Float|Truncate damage))
  (bind _returnvalue_2 (Effects|SpawnEmitterAttached "/Game/Blood_Splatter/Blood_Particles.Blood_Particles" (Variables|Character|GetMesh) "None" "0, 0,15.000000"))
  (EventDispatchers|BindEventtoOnParticleCollide _returnvalue_2 (delegate Custom|On%20Collide%20Event)))

(event OnTargetPerceptionUpdated(AIPerception)
  (params (Actor :type Actor%20Object%20Reference) (Stimulus :type AI%20Stimulus%20Structure))
  (bind _returnvalue (Utilities|Name|MakeLiteralName "target"))
  (bind _returnvalue_2 (Pawn|GetController))
  (bind _returnvalue_3 (AI|GetBlackboard _returnvalue_2))
  (Utilities|Casting|CastToBP_BasePlayer Actor)
  (if (.bSuccessfullySensed (Utilities|Struct|BreakAIStimulus Stimulus))
    (AI|Components|Blackboard|SetValueasObject _returnvalue_3 _returnvalue Actor)
    (else
      (AI|Components|Blackboard|ClearValue _returnvalue_3 _returnvalue))))

(event Custom|On%20Collide%20Event
  (params (EventName :type Name) (EmitterTime :type Float%20%28single-precision%29) (ParticleTime :type Integer) (Location :type Vector) (Velocity :type Vector) (Direction :type Vector) (Normal :type Vector) (BoneName :type Name) (PhysMat :type Physical%20Material%20Object%20Reference))
  (bind _returnvalue (Rendering|Material|CreateDynamicMaterialInstance "/Game/Blood_Splatter/Blood_Decal_Material.Blood_Decal_Material" "None" "None" :!class /Script/Engine.KismetMaterialLibrary))
  (Rendering|Material|SetScalarParameterValue _returnvalue "Frame" (Math|Conversions|ToFloat(Integer) (Math|Random|RandomInteger 11)) :!class /Script/Engine.MaterialInstanceDynamic)
  (Rendering|Decal|SpawnDecalatLocation _returnvalue (Math|Conversions|ToVector(Float) (Math|Random|RandomFloatinRange 2e+01 5e+01)) Location (Math|Conversions|RotationFromXVector Normal) 8.0))

(event EventBeginPlay)

(event Collision|EventActorBeginOverlap
  (params (OtherActor :type Actor%20Object%20Reference)))

(event EventTick
  (params (DeltaSeconds :type Float%20%28single-precision%29)))

(event EventSetHealth
  (params (newHealth :type Float%20%28single-precision%29)))

(fn ConstructionScript)