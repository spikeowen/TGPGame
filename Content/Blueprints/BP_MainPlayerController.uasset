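; Main player controller Blueprint that relays gameplay updates to the on-screen HUD.
; Each event casts the displayed HUD widget to HUD_BP and forwards health, enemy and player regions, weapon icons and rarity tints.
; Toggle events show or hide the crosshair, sniper scope and ammo display.
; Tick, BeginPlay and the construction script are empty, so the graph only acts when its events are called.
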(event EventBeginPlay)

(event EventTick
  (params (DeltaSeconds :type Float%20%28single-precision%29)))

(event EventUpdateWeaponRarity
  (params (rarity :type Integer))
  (bind _ashud_bp (Utilities|Casting|CastToHUD_BP (Variables|Default|GetDisplayedHUD)))
  (Default|UpdatePrimaryRarityTint _ashud_bp rarity))

(event EventUpdateSecondWeaponRarity
  (params (rarity :type Integer))
  (bind _ashud_bp (Utilities|Casting|CastToHUD_BP (Variables|Default|GetDisplayedHUD)))
  (Default|UpdateSecondaryRarityTint _ashud_bp rarity))

(event EventUpdateHealth
  (params (HealthPercent :type Float%20%28single-precision%29))
  (bind _ashud_bp (Utilities|Casting|CastToHUD_BP (Variables|Default|GetDisplayedHUD)))
  (Default|UpdateHealth _ashud_bp HealthPercent))

(event EventUpdateEnemyRegion
  (bind _ashud_bp (Utilities|Casting|CastToHUD_BP (Variables|Default|GetDisplayedHUD)))
  (Default|UpdateEnemySpawnRegion _ashud_bp (Variables|Default|GetSpawnRegion)))

(event EventUpdatePrimaryWeapon
  (bind _ashud_bp (Utilities|Casting|CastToHUD_BP (Variables|Default|GetDisplayedHUD)))
  (Default|UpdatePrimaryWeaponIcon _ashud_bp (Variables|Default|GetPrimaryIcon)))

(event EventUpdateSecondaryWeapon
  (bind _ashud_bp (Utilities|Casting|CastToHUD_BP (Variables|Default|GetDisplayedHUD)))
  (Default|UpdateSecondaryWeaponIcon _ashud_bp (Variables|Default|GetSecondaryIcon)))

(event EventToggleCrosshair
  (params (hidden :type Boolean))
  (bind _ashud_bp (Utilities|Casting|CastToHUD_BP (Variables|Default|GetDisplayedHUD)))
  (if hidden
    (Default|HideCrosshair _ashud_bp)
    (else
      (Default|ShowCrosshair _ashud_bp))))

(event EventToggleSniperScope
  (params (hidden :type Boolean))
  (bind _ashud_bp (Utilities|Casting|CastToHUD_BP (Variables|Default|GetDisplayedHUD)))
  (if hidden
    (Default|HideSniperScope _ashud_bp)
    (else
      (Default|ShowSniperScope _ashud_bp))))

(event EventToggleAmmoDisplay
  (params (Hidden :type Boolean))
  (bind _ashud_bp (Utilities|Casting|CastToHUD_BP (Variables|Default|GetDisplayedHUD)))
  (Default|ToggleAmmoDisplay _ashud_bp Hidden))

(event EventUpdateCurrentZone
  (bind _ashud_bp (Utilities|Casting|CastToHUD_BP (Variables|Default|GetDisplayedHUD)))
  (Default|UpdatePlayerRegion _ashud_bp (Variables|Default|GetPlayerRegion)))

(fn ConstructionScript)